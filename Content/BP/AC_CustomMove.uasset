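; Actor component that steers its owning Character by messaging its AnimInstance, with navmesh path and focus helpers.
; Move converts a target into a mesh-relative direction vector for Strafe or a yaw delta for CIR, draws debug spheres, and reports type changes to animation.
; FindPath returns synchronous path points plus the second point as next waypoint.
; Focus turns the actor toward a point at a constant interpolation rate.
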(event EventBeginPlay
  (bind _returnvalue (Components|GetOwner))
  (bind (_ascharacter _bsuccess) (Utilities|Casting|CastToCharacter _returnvalue))
  (if _bsuccess
    (Variables|Component|SetOwnChar _ascharacter)
    (Variables|Component|SetOwnAnimInstance (Components|SkeletalMesh|GetAnimInstance (Variables|/Script/Engine.Character|GetMesh (Variables|Component|GetOwnChar))))))

(event EventTick
  (params (DeltaSeconds :type Float%20%28single-precision%29)))

(fn FindPath
  (params (PathEnd :type Vector%20%28by%20ref%29))
  (bind _returnvalue (Class|NavigationSystemV1|FindPathtoLocationSynchronously (Transformation|GetActorLocation (Variables|Component|GetOwnChar)) PathEnd (Variables|Component|GetOwnChar) "/Script/AIModule.NavFilter_AIControllerDefault"))
  (return (Variables|/Script/NavigationSystem.NavigationPath|GetPathPoints _returnvalue) (Utilities|Array|Get(acopy) (Variables|/Script/NavigationSystem.NavigationPath|GetPathPoints _returnvalue) 1)))

(fn Move
  (params (TypeMove :type ETypeMove%20Enum :default "NewEnumerator0") (Target :type Vector))
  (Utilities|FlowControl|Sequence
    (:then_0
      (switch Utilities|FlowControl|Switch|SwitchonETypeMove TypeMove
        (:NewEnumerator0
          (bind _output_get (Variables|Info|SetVectorToTarget (Math|Vector|GetForwardVector (Math|Rotator|Delta(Rotator) (Math|Rotator|Delta(Rotator) (Utilities|LookatRot Target) (Transformation|GetActorRotation (Variables|Component|GetOwnChar))) (|RotMeshOwner)))))
          (Class|BPIMovementABP|NewVector(Message) (Variables|Component|GetOwnAnimInstance) _output_get)
          (Rendering|Debug|DrawDebugSphere Target 75.0 12 "(R=1.000000,G=0.000000,B=0.010882,A=1.000000)" (Class|ActorComponent|GetComponentTickInterval) 0.5))
        (:NewEnumerator1
          (bind _output_get_2 (Variables|Info|SetRot%20Z (.Yaw (Math|Rotator|BreakRotator (Math|Rotator|Delta(Rotator) (Utilities|LookatRot Target) (Transformation|GetActorRotation (Variables|Component|GetOwnChar)))))))
          (Class|BPIMovementABP|NewDir(Message) (Variables|Component|GetOwnAnimInstance) _output_get_2)
          (Rendering|Debug|DrawDebugSphere Target 5e+01 8 "(R=0.206559,G=0.000000,B=1.000000,A=1.000000)" (Class|ActorComponent|GetComponentTickInterval) 0.5))))
    (:then_1
      (CallFunction|UpdateMove TypeMove)
      (return (Variables|Info|GetVectorToTarget) (Variables|Info|GetRot%20Z)))))

(fn Focus
  (params (PointFocus :type Vector) (Tick%28DeltaTime%29 :type Float%20%28double-precision%29) (InterpSpeed :type Float%20%28single-precision%29))
  (Transformation|SetActorRotation (Variables|Component|GetOwnChar) (Class|KismetMathLibrary|RInterptoConstant (Transformation|GetActorRotation (Variables|Component|GetOwnChar)) (Utilities|LookatRot PointFocus) Tick%28DeltaTime%29 InterpSpeed)))

(fn UpdateMove
  (params (TMove :type ETypeMove%20Enum :default "NewEnumerator0"))
  (if (Utilities|Enum|NotEqual(Enum) TMove (Variables|Info|GetCTypeMove))
    (Variables|Info|SetCTypeMove TMove)
    (Class|BPIMovementABP|InfoStates(Message) (Variables|Component|GetOwnAnimInstance) (Variables|Info|GetCTypeMove))))